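; BP_Construct is an actor that procedurally builds a grid of static mesh cubes with randomized heights.
; Its construction script loops over ISizeX and ISizeY, adding a Cube mesh component per cell with a random Z scale, re-rolled on each construction.
; GetLocation spaces cells by FCubeSize plus FCubeJit and offsets them by half the grid extent, roughly centering it on the actor.
; The event graph holds no active logic.
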(event EventBeginPlay)

(event Collision|EventActorBeginOverlap
  (params (OtherActor :type Actor%20Object%20Reference)))

(event EventTick
  (params (DeltaSeconds :type Float%20%28single-precision%29)))

(fn ConstructionScript
  (bind _i_sizex (Variables|Default|Geti_SizeX))
  (bind _i_sizey (Variables|Default|Geti_SizeY))
  (for _index (range 1 _i_sizey)
    (for _index_2 (range 1 _i_sizex)
      (bind _returnvalue (AddComponent|AddStaticMeshComponent false (Math|Transform|MakeTransform (Math|Vector|MakeVector (CallFunction|GetLocation _index_2 (Math|Conversions|ToFloat(Integer) _i_sizex)) (CallFunction|GetLocation _index (Math|Conversions|ToFloat(Integer) _i_sizey)) 0.0) "0, 0, 0" (Math|Vector|MakeVector 1.0 1.0 (Math|Random|RandomFloatinRange 0.1 0.3)))))
      (Components|StaticMesh|SetStaticMesh _returnvalue "/Game/Models/Cube.Cube"))))

(fn GetLocation
  (params (i_Index :type Integer) (i_Size :type Float%20%28single-precision%29))
  (return (- (* (+ (Variables|Default|Getf_CubeSize) (Variables|Default|Getf_CubeJit)) i_Index) (* i_Size (+ (Variables|Default|Getf_CubeSize) (Variables|Default|Getf_CubeJit)) 0.5))))